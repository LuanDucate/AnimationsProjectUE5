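; Actor component that gives its owning Character a dodge roll.
; On BeginPlay it caches the owner as a Character and clears the rolling flag.
; The IA_Dodge input plays a forward roll montage on the character's mesh, using the flag to block new rolls during playback.
; The flag clears only when the montage completes, with no handling for interruption.
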(event Input|EnhancedActionEvents|EnhancedInputActionIA_Dodge
  (params (ActionValue :type Boolean) (ElapsedSeconds :type Float%20%28double-precision%29) (TriggeredSeconds :type Float%20%28double-precision%29) (InputAction :type Input%20Action%20Object%20Reference :default "/Game/Input/Actions/IA_Dodge.IA_Dodge"))
  (:Started
    (if (not (Variables|Default|GetIsRolling))
      (Animation|Montage|PlayMontage (Variables|/Script/Engine.Character|GetMesh (Variables|Default|GetRefCharacter)) "/Game/Characters/Mannequins/Anims/Roll/A_Roll_IdleFwd_Montage.A_Roll_IdleFwd_Montage"
        (:then
          (Variables|Default|SetIsRolling true))
        (:OnCompleted
          (Variables|Default|SetIsRolling false))))))

(event EventBeginPlay
  ;[0.15 0.15 0.15 0.5] Get Character Reference
  (bind _ascharacter (Utilities|Casting|CastToCharacter (Components|GetOwner)))
  (Variables|Default|SetRefCharacter _ascharacter)
  (Variables|Default|SetIsRolling false))